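; BP_WrapZone is a trigger zone that wraps the player spaceship to another position in the level, driven by a TargetActor reference.
; When a BP_SpaceShip begins overlapping TriggerBox, it moves to the target's coordinate on one axis and keeps the other.
; IsHorizontal selects the replaced axis (Y when true, X otherwise), and height is forced to a fixed Z without sweeping.
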(event OnComponentBeginOverlap(TriggerBox)
  (params (OverlappedComponent :type Primitive%20Component%20Object%20Reference) (OtherActor :type Actor%20Object%20Reference) (OtherComp :type Primitive%20Component%20Object%20Reference) (OtherBodyIndex :type Integer) (bFromSweep :type Boolean) (SweepResult :type Hit%20Result%20Structure%20%28by%20ref%29))
  (bind _asbp_space_ship (Utilities|Casting|CastToBP_SpaceShip OtherActor))
  (if (Variables|Default|GetIsHorizontal)
    (Transformation|SetActorLocation _asbp_space_ship (Math|Vector|MakeVector (.x (Transformation|GetActorLocation _asbp_space_ship)) (.y (Transformation|GetActorLocation (Variables|Default|GetTargetActor))) 1e+02) false false)
    (else
      (Transformation|SetActorLocation _asbp_space_ship (Math|Vector|MakeVector (.x (Transformation|GetActorLocation (Variables|Default|GetTargetActor))) (.y (Transformation|GetActorLocation _asbp_space_ship)) 1e+02) false false))))

(event EventBeginPlay)

(event Collision|EventActorBeginOverlap
  (params (OtherActor :type Actor%20Object%20Reference)))

(event EventTick
  (params (DeltaSeconds :type Float%20%28single-precision%29)))

(fn ConstructionScript)